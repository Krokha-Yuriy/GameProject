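; SpaceControll is a controller that spawns and possesses the character skin the player selected.
; On BeginPlay it loads a BP_EndlesSaveGame from a save slot, then spawns the class at the saved SelectSkin index of its Char array at the first PlayerStart found.
; BlurGo, BlurStop, FireGo and FireStop are stubs that only return false.
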(event `self.ReceiveBeginPlay`
  (bind _returnvalue (`GameplayStatics.LoadGameFromSlot` (`self.Slot Name`)))
  (bind _asbp_endles_save_game (cast `/Game/Widgets/BP_EndlesSaveGame` _returnvalue))
  (`self.Spawn`))

(event `Spawn`
  (bind _outactors (`GameplayStatics.GetAllActorsOfClass` "/Script/Engine.PlayerStart"))
  (set `self.Start Player` _outactors)
  (bind _returnvalue (`|SpawnActorFromClass` (`|GetArrayItem` (`/Game/Widgets/BP_EndlesSaveGame.Char` (stale `self.ReceiveBeginPlay` _asbp_endles_save_game)) (`/Game/Widgets/BP_EndlesSaveGame.SelectSkin` (stale `self.ReceiveBeginPlay` _asbp_endles_save_game))) (`self.GetTransform` (`|GetArrayItem` (`self.Start Player`))) "Undefined" "OverrideRootScale" null null))
  (`self.Possess` _returnvalue))

(fn `BlurGo`
  (returns (`Blur+` :type Boolean))
  (return false))

(fn `BlurStop`
  (returns (`Blur-` :type Boolean))
  (return false))

(fn `FireGo`
  (returns (Fire :type Boolean))
  (return false))

(fn `FireStop`
  (returns (`Stop?` :type Boolean))
  (return false))

(fn `UserConstructionScript`)