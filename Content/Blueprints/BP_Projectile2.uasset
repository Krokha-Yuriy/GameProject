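; BP_Projectile2 is a short-lived projectile that damages BP_PyrEnemy actors and self-destructs two seconds after BeginPlay.
; Its Box overlap casts to that enemy, skips it if it is its own owner, then applies damage and destroys the projectile.
; A random pick then spawns a small fire explosion at its location, though RandomInteger(2) never reaches the third effect, Fire_Exp_01.
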(event `self.Box.OnComponentBeginOverlap`
  (params (OverlappedComponent :type "PrimitiveComponent Object Reference") (OtherActor :type "Actor Object Reference") (OtherComp :type "PrimitiveComponent Object Reference") (OtherBodyIndex :type Integer) (bFromSweep :type Boolean) (SweepResult :type "HitResult Structure (by ref)"))
  (bind _asbp_pyr_enemy (cast `/Game/Assets/Enemies/BP_PyrEnemy` OtherActor))
  (if (not (== OtherActor (`self.GetOwner` _asbp_pyr_enemy)))
    (`GameplayStatics.ApplyDamage` OtherActor 1.0)
    (`self.K2_DestroyActor`)
    (bind _output_get (set `self.ExplosionRandom` (`KismetMathLibrary.RandomInteger` 2)))
    (if (== _output_get 0)
      (`GameplayStatics.SpawnEmitterAtLocation` "/Game/Assets/M5VFXVOL2/Particles/Explosion/Fire_Exp_03.Fire_Exp_03" (`self.K2_GetActorLocation`) (struct) (0.1 0.1 0.1))
      (elif (== (`self.ExplosionRandom`) 1)
        (`GameplayStatics.SpawnEmitterAtLocation` "/Game/Assets/M5VFXVOL2/Particles/Explosion/Fire_Exp_00.Fire_Exp_00" (`self.K2_GetActorLocation`) (struct) (0.1 0.1 0.1))
        (elif (== (`self.ExplosionRandom`) 2)
          (`GameplayStatics.SpawnEmitterAtLocation` "/Game/Assets/M5VFXVOL2/Particles/Explosion/Fire_Exp_01.Fire_Exp_01" (`self.K2_GetActorLocation`) (struct) (0.1 0.1 0.1)))))))

(event `self.ReceiveBeginPlay`
  (`KismetSystemLibrary.Delay` 2.0)
  (`self.K2_DestroyActor`))

(fn `UserConstructionScript`)