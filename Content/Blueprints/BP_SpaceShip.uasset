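; Player spaceship that flies on horizontal and vertical axes, auto-fires projectiles from two points and opens the pause menu.
; Looping random timers periodically stall the guns by stretching the shared fire delay and apply a temporary camera blur post-process.
; Both glitches are broadcast to BPI_FireStop actors, while getter functions expose fire delay, guns and speed.
; Damage decrements HP; at zero the ship explodes randomly and calls the MultiControll controller's Spawn.
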(event `self.ReceiveBeginPlay`
  (`|ExecutionSequence`
    (:`then_0`
      ;[1 1 1] Fire
      (`KismetSystemLibrary.Delay` (`self.Duration`))
      (`self.Fire`)
      (`self.Fire2`))
    (:`then_1`
      ;[1 1 1] StopFire
      (bind _outactors (`GameplayStatics.GetAllActorsWithInterface` "/Game/Interfaces/BPI_FireStop.BPI_FireStop_C"))
      (bind _output_get (set `self.Out Actors` _outactors))
      (bind _output_get_2 (set `self.DelayBetweenGunOff` (`KismetMathLibrary.RandomFloatInRange` 30.0 40.0)))
      (`KismetSystemLibrary.Delay` _output_get_2)
      (message `/Game/Interfaces/BPI_FireStop.FireStop` _output_get :!label _label)
      (bind _output_get_3 (set `self.Duration` (`KismetMathLibrary.RandomFloatInRange` 2.0 4.0)))
      (`KismetSystemLibrary.Delay` _output_get_3)
      (message `/Game/Interfaces/BPI_FireStop.FireGo` (`self.Out Actors`))
      (set `self.Duration` 0.6)
      (bind _output_get_4 (set `self.DelayBetweenGunOff` (`KismetMathLibrary.RandomFloatInRange` 30.0 40.0)))
      (`KismetSystemLibrary.Delay` _output_get_4)
      (for _ (range 1)
        (goto _label)))
    (:`then_2`
      ;[1 1 1] Blur
      (bind _output_get_5 (set `self.DelayBetweenBlur` (`KismetMathLibrary.RandomFloatInRange` 80.0 90.0) :!label _label_2))
      (`KismetSystemLibrary.Delay` _output_get_5)
      (message `/Game/Interfaces/BPI_FireStop.BlurGo` (`self.Out Actors`))
      (`self.Blur`)
      (for _ (range 1)
        (goto _label_2)))))

(event `InputAxis|MoveRightLeft`
  (params (AxisValue :type "Float (single-precision)"))
  ;[1 1 1] Right/Left movement
  (`self.AddMovementInput` (`self.GetActorRightVector`) AxisValue))

(event `InputAxis|MoveTopDown`
  (params (AxisValue :type "Float (single-precision)"))
  ;[1 1 1] Top/Down movement
  (`self.AddMovementInput` (0.0 0.0 1.0) AxisValue))

(event `Fire`
  ;[1 1 1] Fire
  (`|SpawnActorFromClass` "/Game/Blueprints/BP_Projectile1.BP_Projectile1_C" (`SceneComponent.K2_GetComponentToWorld` (`self.Scene`)) "Undefined" "OverrideRootScale" self null)
  (`KismetSystemLibrary.Delay` (`self.Duration`))
  (`self.Fire`)
  (`GameplayStatics.SpawnSound2D` "/Game/Sounds/projectile.projectile" 0.01 1.0 0.0 null false false :!label _label_3))

(event `Fire2`
  ;[1 1 1] Fire
  (`|SpawnActorFromClass` "/Game/Blueprints/BP_Projectile1.BP_Projectile1_C" (`SceneComponent.K2_GetComponentToWorld` (`self.Scene1`)) "Undefined" "OverrideRootScale" self null)
  (`KismetSystemLibrary.Delay` (`self.Duration`))
  (`self.Fire2`)
  (goto _label_3))

(event `Blur`
  ;[1 1 1] Blur
  (`CameraComponent.AddOrUpdateBlendable` (`self.Camera`) (`self.BlurMaterial`) 1.0)
  (bind _output_get (set `self.BlurTime` (`KismetMathLibrary.RandomFloatInRange` 3.0 5.0)))
  (`KismetSystemLibrary.Delay` _output_get)
  (`CameraComponent.RemoveBlendable` (`self.Camera`) (`self.BlurMaterial`))
  (message `/Game/Interfaces/BPI_FireStop.BlurStop` (`self.Out Actors`)))

(event `InputAction|PauseMenu`
  (params (Key :type "Key Structure"))
  (bind _returnvalue (`GameplayStatics.GetPlayerController` 0))
  (:`Pressed`
    (`GameplayStatics.SetGamePaused` true)
    (`self.DisableInput` _returnvalue)
    (set `PlayerController.bShowMouseCursor` true _returnvalue)
    (bind _returnvalue_2 (`|CreateWidget` "/Game/Widgets/WidgetBluePrints/WB_MenuPaused.WB_MenuPaused_C" _returnvalue))
    (`UserWidget.AddToViewport` _returnvalue_2 0)
    (`WidgetBlueprintLibrary.SetInputMode_UIOnlyEx` _returnvalue null)))

(event `self.ReceiveAnyDamage`
  (params (Damage :type "Float (single-precision)") (DamageType :type "DamageType Object Reference") (InstigatedBy :type "Controller Object Reference") (DamageCauser :type "Actor Object Reference"))
  (bind _returnvalue (`GameplayStatics.GetPlayerController` 0))
  (bind _result (`/Engine/EditorBlueprintResources/StandardMacros.DecrementFloat` (`self.MaxHP`))
    (:`  `
      (set `self.CurrentHP` _result)
      (if (== 0.0 (`self.CurrentHP`))
        (`GameplayStatics.SpawnSound2D` "/Game/Sounds/enemydestroyed.enemydestroyed" 0.1 1.0 0.0 null false false)
        (`self.K2_DestroyActor`)
        (`/Game/GameMode/MultiGame/MultiControll.Spawn` (cast `/Game/GameMode/MultiGame/MultiControll` _returnvalue :!pure true) _returnvalue)
        (bind _output_get (set `self.ExplosionRandom` (`KismetMathLibrary.RandomIntegerInRange` 0 2)))
        (if (== _output_get 0)
          (`GameplayStatics.SpawnEmitterAtLocation` "/Game/Assets/M5VFXVOL2/Particles/Explosion/Fire_Exp_03.Fire_Exp_03" (`self.K2_GetActorLocation`))
          (elif (== (`self.ExplosionRandom`) 1)
            (`GameplayStatics.SpawnEmitterAtLocation` "/Game/Assets/M5VFXVOL2/Particles/Explosion/Fire_Exp_00.Fire_Exp_00" (`self.K2_GetActorLocation`))
            (elif (== (`self.ExplosionRandom`) 2)
              (`GameplayStatics.SpawnEmitterAtLocation` "/Game/Assets/M5VFXVOL2/Particles/Explosion/Fire_Exp_01.Fire_Exp_01" (`self.K2_GetActorLocation`)))))))))

(fn `BlurGo`
  (returns (`Blur+` :type Boolean))
  (return false))

(fn `BlurStop`
  (returns (`Blur-` :type Boolean))
  (return false))

(fn `FireGo`
  (returns (Fire :type Boolean))
  (return false))

(fn `FireStop`
  (returns (`Stop?` :type Boolean))
  (return false))

(fn `GetDuration`
  (returns (Duration :type "Float (double-precision)"))
  (return (`self.Duration`)))

(fn `GetGans`
  (returns (Gans :type "Float (double-precision)"))
  (return (`self.Gans`)))

(fn `GetMinutes`
  (returns (Minut :type Integer))
  (return 0))

(fn `GetSeconds`
  (returns (Sec :type Integer))
  (return 0))

(fn `GetSpeed`
  (returns (Speed :type "Float (double-precision)"))
  (return (`CharacterMovementComponent.MaxFlySpeed` (`self.CharacterMovement`))))

(fn `UserConstructionScript`)