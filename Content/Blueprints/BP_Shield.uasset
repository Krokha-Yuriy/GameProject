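; BP_Shield is a destructible shield actor whose hit points come from the player's save game.
; On BeginPlay it loads the BP_EndlesSaveGame slot and copies ShildMaxHP into MaxHP, which serves as remaining health.
; AnyDamage subtracts from MaxHP, then plays a 2D destruction sound and destroys the actor only when the value equals exactly zero.
; The IsDead function is an empty stub.
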(event `self.ReceiveBeginPlay`
  (bind _returnvalue (`GameplayStatics.LoadGameFromSlot` (`self.Save slot`)))
  (bind _asbp_endles_save_game (cast `/Game/Widgets/BP_EndlesSaveGame` _returnvalue))
  (set `self.MaxHP` (`KismetMathLibrary.Conv_IntToDouble` (`/Game/Widgets/BP_EndlesSaveGame.ShildMaxHP` _asbp_endles_save_game))))

(event `self.ReceiveAnyDamage`
  (params (Damage :type "Float (single-precision)") (DamageType :type "DamageType Object Reference") (InstigatedBy :type "Controller Object Reference") (DamageCauser :type "Actor Object Reference"))
  (set `self.MaxHP` (- (`self.MaxHP`) (`self.Damage`)))
  (if (== 0.0 (`self.MaxHP`))
    (`GameplayStatics.SpawnSound2D` "/Game/Sounds/shielddestroyed.shielddestroyed" 0.3 1.0 0.0 null false false)
    (`self.K2_DestroyActor`)))

(event `self.ReceiveTick`
  (params (DeltaSeconds :type "Float (single-precision)")))

(fn `IsDead`)

(fn `UserConstructionScript`)