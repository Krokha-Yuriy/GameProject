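; Game-over handler that ends a run, saves progress and shows the death screen.
; Tick watches the IsDead flag, which NewBoll sets, and calls EndGame after a short Delay.
; EndGame pauses the game, then creates or updates BP_EndlesSaveGame with GameModeTest's score if it is a new high, banking saved Coins only for existing saves.
; It finally displays WB_DeadScreen with the cursor and UI-only input.
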(event `self.ReceiveBeginPlay`)

(event `self.ReceiveTick`
  (params (DeltaSeconds :type "Float (single-precision)"))
  (if (`self.is dead`)
    (`KismetSystemLibrary.Delay` 3.0)
    (`self.EndGame`)))

(fn `EndGame`
  (bind _returnvalue (`GameplayStatics.GetPlayerController` 0))
  (bind _saveslot (`self.SaveSlot`))
  (bind _saveslot_2 (`self.SaveSlot`))
  (bind _saveref (`self.SaveRef`))
  (`GameplayStatics.SetGamePaused` true)
  (bind _asgame_mode_test (cast `/Game/Level_1/GameModeTest` (`GameplayStatics.GetGameMode`)))
  (bind _returnvalue_2 (`GameplayStatics.DoesSaveGameExist` _saveslot))
  (if _returnvalue_2
    (bind _returnvalue_3 (`GameplayStatics.LoadGameFromSlot` _saveslot))
    (bind _output_get (set `self.SaveRef` _returnvalue_3))
    (bind _asbp_endles_save_game (cast `/Game/Widgets/BP_EndlesSaveGame` _output_get))
    (bind _currentpoint (`/Game/Level_1/GameModeTest.CurrentPoint` _asgame_mode_test))
    (if (> _currentpoint (`/Game/Widgets/BP_EndlesSaveGame.HighsCoreValue` _asbp_endles_save_game))
      (bind _coins (`/Game/Widgets/BP_EndlesSaveGame.Coins` _asbp_endles_save_game))
      (set `/Game/Widgets/BP_EndlesSaveGame.CurrentCoins` (+ (`/Game/Widgets/BP_EndlesSaveGame.CurrentCoins` _asbp_endles_save_game) _coins) _asbp_endles_save_game)
      (set `/Game/Widgets/BP_EndlesSaveGame.HighsCoreValue` _currentpoint _asbp_endles_save_game)
      (`GameplayStatics.SaveGameToSlot` _saveref _saveslot_2)
      (else
        (set `/Game/Widgets/BP_EndlesSaveGame.CurrentCoins` (+ (`/Game/Widgets/BP_EndlesSaveGame.CurrentCoins` _asbp_endles_save_game) _coins) _asbp_endles_save_game)
        (`GameplayStatics.SaveGameToSlot` _saveref _saveslot_2)))
    (else
      (bind _returnvalue_4 (`GameplayStatics.CreateSaveGameObject` "/Game/Widgets/BP_EndlesSaveGame.BP_EndlesSaveGame_C"))
      (bind _output_get_2 (set `self.SaveRef` _returnvalue_4))
      (bind _asbp_endles_save_game_2 (cast `/Game/Widgets/BP_EndlesSaveGame` _output_get_2))
      (set `/Game/Widgets/BP_EndlesSaveGame.HighsCoreValue` _currentpoint _asbp_endles_save_game_2)
      (`GameplayStatics.SaveGameToSlot` _saveref _saveslot_2)))
  (set `PlayerController.bShowMouseCursor` true _returnvalue)
  (bind _returnvalue_5 (`|CreateWidget` "/Game/Widgets/WidgetBluePrints/WB_DeadScreen.WB_DeadScreen_C" _returnvalue))
  (`UserWidget.AddToViewport` _returnvalue_5 0)
  (`WidgetBlueprintLibrary.SetInputMode_UIOnlyEx` (`GameplayStatics.GetPlayerController` 0) _returnvalue_5))

(fn `IsDead`
  (returns (NewParam :type Boolean))
  (return false))

(fn `NewBoll`
  (returns (NewParam :type Boolean))
  (set `self.is dead` true)
  (return false))

(fn `UserConstructionScript`)