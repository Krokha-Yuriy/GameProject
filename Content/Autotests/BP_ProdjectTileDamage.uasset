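; BP_ProdjectTileDamage is an automated functional test whose name points to projectile damage testing, but it is unfinished.
; On test start it waits briefly and looks up a BP_Projectile1 actor, with no check or finish call after that.
; Disconnected pass/fail nodes remain, with messages about comparing station max HP to a saved value, so they never execute.
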(event `self.ReceiveStartTest`
  (`KismetSystemLibrary.Delay` 0.2)
  (`GameplayStatics.GetActorOfClass` "/Game/Blueprints/BP_Projectile1.BP_Projectile1_C"))

(fn `UserConstructionScript`
  (`parent.UserConstructionScript`))