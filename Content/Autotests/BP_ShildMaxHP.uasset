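; BP_ShildMaxHP is a functional autotest that checks that the shield's max HP matches the value stored in the save game.
; After a short delay on test start, it finds the BP_Shield actor and loads the save slot as BP_EndlesSaveGame.
; It succeeds when MaxHP equals the saved ShildMaxHP, and fails on a mismatch or a failed save cast.
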(event `self.ReceiveStartTest`
  (bind _returnvalue (`KismetSystemLibrary.GetDisplayName` self))
  (`KismetSystemLibrary.Delay` 0.2)
  (bind _returnvalue_2 (`GameplayStatics.GetActorOfClass` "/Game/Blueprints/BP_Shield.BP_Shield_C"))
  (bind _returnvalue_3 (`GameplayStatics.LoadGameFromSlot` (`self.Save slot`)))
  (bind _asbp_endles_save_game (cast `/Game/Widgets/BP_EndlesSaveGame` _returnvalue_3)
    (:`then`
      (if (== (`/Game/Blueprints/BP_Shield.MaxHP` _returnvalue_2) (`/Game/Widgets/BP_EndlesSaveGame.ShildMaxHP` _asbp_endles_save_game))
        (`self.FinishTest` "Succeeded" (`KismetStringLibrary.Concat_StrStr` "Test passed:" _returnvalue))
        (else
          (`self.FinishTest` "Failed" (`KismetStringLibrary.Concat_StrStr` "Shild Max HP in not equal save Max HP" _returnvalue)))))
    (:`CastFailed`
      (`self.FinishTest` "Failed" "Cast to save is faided"))))

(fn `UserConstructionScript`
  (`parent.UserConstructionScript`))