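; BP_Spawn is an enemy spawner that continuously spawns enemies at its own location in escalating type order.
; BeginPlay runs a delayed loop whose wave counter selects successive bands of Pyr, Arach, Tank and Mecha enemies, then resets to repeat the cycle.
; Tick uses a ten-second delay to step RespawnTime down while it exceeds a two-second threshold, speeding up spawning over time.
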(event `self.ReceiveBeginPlay`
  (set `self.Waves` 0 :!label _label)
  (`|SpawnActorFromClass` "/Game/Assets/Enemies/BP_PyrEnemy.BP_PyrEnemy_C" (`KismetMathLibrary.MakeTransform` (`self.K2_GetActorLocation`)) "Undefined" "OverrideRootScale" null null :!label _label_2)
  (`KismetSystemLibrary.Delay` (`self.RespawnTime`))
  (set `self.Waves` (+ (`self.Waves`) 1))
  (for _ (range 1)
    (if (`KismetMathLibrary.InRange_IntInt` (`self.Waves`))
      (goto _label_2)
      (else
        (`|SpawnActorFromClass` "/Game/Assets/Enemies/BP_ArachEnemy.BP_ArachEnemy_C" (`KismetMathLibrary.MakeTransform` (`self.K2_GetActorLocation`)) "Undefined" "OverrideRootScale" null null :!label _label_3)
        (`KismetSystemLibrary.Delay` (`self.RespawnTime`))
        (set `self.Waves` (+ (`self.Waves`) 1))
        (for _ (range 1)
          (if (`KismetMathLibrary.InRange_IntInt` (`self.Waves`) 11 21)
            (goto _label_3)
            (else
              (`|SpawnActorFromClass` "/Game/Assets/Enemies/BP_TankEnemy.BP_TankEnemy_C" (`KismetMathLibrary.MakeTransform` (`self.K2_GetActorLocation`)) "Undefined" "OverrideRootScale" null null :!label _label_4)
              (`KismetSystemLibrary.Delay` (`self.RespawnTime`))
              (set `self.Waves` (+ (`self.Waves`) 1))
              (for _ (range 1)
                (if (`KismetMathLibrary.InRange_IntInt` (`self.Waves`) 22 32)
                  (goto _label_4)
                  (else
                    (`|SpawnActorFromClass` "/Game/Assets/Enemies/BP_MechaEnemy.BP_MechaEnemy_C" (`KismetMathLibrary.MakeTransform` (`self.K2_GetActorLocation`)) "Undefined" "OverrideRootScale" null null :!label _label_5)
                    (`KismetSystemLibrary.Delay` (`self.RespawnTime`))
                    (set `self.Waves` (+ (`self.Waves`) 1))
                    (for _ (range 1)
                      (if (`KismetMathLibrary.InRange_IntInt` (`self.Waves`) 33 43)
                        (goto _label_5)
                        (else
                          (goto _label))))))))))))))

(event `self.ReceiveTick`
  (params (DeltaSeconds :type "Float (single-precision)"))
  (if (> (`self.RespawnTime`) 2.0) :!label _label_6
    (`KismetSystemLibrary.Delay` 10.0)
    (set `self.RespawnTime` (- (`self.RespawnTime`) 1.0))
    (for _ (range 1)
      (goto _label_6))))

(fn `UserConstructionScript`)