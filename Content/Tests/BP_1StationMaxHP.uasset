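; Functional test that checks the station's max HP stored in the save game.
; On test start it waits briefly, loads the SaveSlot save and reads station max HP from it through an interface message.
; It passes and logs the value if that exactly matches a hard-coded expected number, otherwise it fails with a mismatch message.
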(event `self.ReceiveStartTest`
  (bind _returnvalue (`KismetSystemLibrary.GetDisplayName` self))
  (`KismetSystemLibrary.Delay` 0.2)
  (bind _returnvalue_2 (`GameplayStatics.LoadGameFromSlot` (`self.Save slot`)))
  (bind _savestationhp (message `/Game/Interfaces/BPI_TestSave.GetSaveStationMaxHP` _returnvalue_2))
  (if (== 50.0 _savestationhp)
    (`self.LogMessage` (`KismetStringLibrary.Concat_StrStr` "Station max HP: " (`KismetStringLibrary.Conv_IntToString` _savestationhp)))
    (`self.FinishTest` "Succeeded" (`KismetStringLibrary.Concat_StrStr` "Test passed:" _returnvalue))
    (else
      (`self.FinishTest` "Failed" (`KismetStringLibrary.Concat_StrStr` "Station Max HP in not equal save Max HP" _returnvalue)))))

(fn `UserConstructionScript`
  (`parent.UserConstructionScript`))