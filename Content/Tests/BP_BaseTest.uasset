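; Base functional test Blueprint that provides shared setup and shutdown behavior for automated game tests.
; PrepareTest builds the timeout message from the test's display name, and IsReady waits until player character 0 is valid.
; OnAutoTestFinished optionally quits the game, while the save getters for shield and station max HP are stubs returning zero.
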(event `self.ReceivePrepareTest`
  (set `self.TimesUpMessage` (`KismetTextLibrary.Conv_StringToText` (`KismetStringLibrary.Concat_StrStr` "Times up:" (`KismetSystemLibrary.GetDisplayName` self)))))

(fn `GetSaveShildMaxHP`
  (returns (SaveShildHP :type Integer))
  (return 0))

(fn `GetSaveStationMaxHP`
  (returns (SaveStationHP :type Integer))
  (return 0))

(fn `IsReady`
  (returns (ReturnValue :type Boolean))
  (return (`KismetSystemLibrary.IsValid` (`GameplayStatics.GetPlayerCharacter` 0))))

(fn `OnAutoTestFinished`
  (params (`Quit game` :type Boolean))
  (if `Quit game`
    (`KismetSystemLibrary.QuitGame` null "Quit")))

(fn `UserConstructionScript`)