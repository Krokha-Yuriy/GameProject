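; BP_StationHPtest is a functional test that checks the station max HP stored in a save game.
; It reports ready once the player character is valid.
; On start, it waits briefly, loads save slot "1" and reads the max HP through GetSaveStationMaxHPMessage.
; It passes only if that value equals the hard-coded expected amount, otherwise it fails.
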(event `self.ReceiveStartTest`
  (`KismetSystemLibrary.Delay` 0.1)
  (bind _returnvalue (`GameplayStatics.LoadGameFromSlot` "1"))
  (bind _savestationhp (message `/Game/Interfaces/BPI_TestSave.GetSaveStationMaxHP` _returnvalue))
  (if (== _savestationhp 25)
    (`self.FinishTest` "Succeeded" "Station HP test successfull")
    (else
      (`self.FinishTest` "Failed" "Station HP test failed"))))

(fn `IsReady`
  (returns (ReturnValue :type Boolean))
  (return (`KismetSystemLibrary.IsValid` (`GameplayStatics.GetPlayerCharacter` 0))))

(fn `UserConstructionScript`)