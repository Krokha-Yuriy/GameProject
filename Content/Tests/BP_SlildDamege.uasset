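; BP_SlildDamege is a functional test that checks for an actor hit and reports shield HP after damage.
; On overlap it gets an actor from the overlap's actor through a message call, logs that actor's shield HP, destroys it and finishes as Succeeded.
; The test passes on any overlap without comparing the HP value.
; Its own GetActor and GetShildHP functions are empty stubs, and the prepare, start and tick events are disabled.
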(event `self.Actor.OnActorBeginOverlap`
  (params (OverlappedActor :type "Actor Object Reference") (OtherActor :type "Actor Object Reference"))
  (bind _actor (message `/Game/Interfaces/BPI_Test.GetActor` OverlappedActor))
  (bind _shildhp (message `/Game/Interfaces/BPI_Test.GetShildHP` _actor))
  (`self.LogMessage` (`KismetStringLibrary.Concat_StrStr` "Shild HP after damege:" (`KismetStringLibrary.Conv_DoubleToString` _shildhp)))
  (`self.K2_DestroyActor` _actor)
  (`self.FinishTest` "Succeeded" "Actor Hit"))

(fn `GetActor`
  (returns (Actor :type "Actor Object Reference"))
  (return null))

(fn `GetShildHP`
  (returns (ShildHP :type "Float (double-precision)"))
  (return 0.0))

(fn `IsReady`
  (returns (ReturnValue :type Boolean))
  (bind _returnvalue (`parent.IsReady`))
  (return _returnvalue))

(fn `UserConstructionScript`
  (`parent.UserConstructionScript`))