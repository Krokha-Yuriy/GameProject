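; Functional test that checks a shield loses exactly one HP when damaged.
; IsReady waits for a valid player character; StartTest is empty, so the actor's begin-overlap event drives the check.
; It reads shield HP from OverlappedActor and passes if it equals the saved max minus one from slot "1", failing otherwise or if the save cast fails.
; A CheckEnemy helper for tagged actors is defined but never called here.
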(event `self.ReceiveStartTest`)

(event `self.Actor.OnActorBeginOverlap`
  (params (OverlappedActor :type "Actor Object Reference") (OtherActor :type "Actor Object Reference"))
  (bind _shildhp (message `/Game/Interfaces/BPI_Test.GetShildHP` OverlappedActor))
  (bind _returnvalue (`KismetStringLibrary.Conv_DoubleToString` _shildhp))
  (`KismetSystemLibrary.PrintString` _returnvalue)
  (`self.LogMessage` _returnvalue)
  (bind _returnvalue_2 (`GameplayStatics.LoadGameFromSlot` "1"))
  (bind _asbp_endles_save_game (cast `/Game/Widgets/BP_EndlesSaveGame` _returnvalue_2)
    (:`then`
      (if (== _shildhp (- (`/Game/Widgets/BP_EndlesSaveGame.ShildMaxHP` _asbp_endles_save_game) 1))
        (`self.FinishTest` "Succeeded" "Damage is valid")
        (else
          (`self.FinishTest` "Failed" "Damage  is not valid"))))
    (:`CastFailed`
      (`self.FinishTest` "Failed" "No shield"))))

(fn `CheckEnemy`
  (params (Tag :type Name))
  (bind _outactors (`GameplayStatics.GetAllActorsWithTag` Tag))
  (for _array_element _outactors
    (`/Engine/EditorBlueprintResources/StandardMacros.IsValid` _array_element
      (:`Is Valid`
        (`KismetSystemLibrary.PrintString` "Enemy spawned"))
      (:`Is Not Valid`
        (`self.FinishTest` "Failed" "Cant find enemy")))))

(fn `IsReady`
  (returns (ReturnValue :type Boolean))
  (return (`KismetSystemLibrary.IsValid` (`GameplayStatics.GetPlayerCharacter` 0))))

(fn `UserConstructionScript`)