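; Functional test that checks whether the saved shield max HP matches the expected value.
; It reports ready once the player character is valid, then waits briefly and loads the save game from a fixed slot.
; It reads the value through a getter message on the save object and finishes as succeeded or failed against a hardcoded number, without writing any save data itself.
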(event `self.ReceiveStartTest`
  (`KismetSystemLibrary.Delay` 0.1)
  (bind _returnvalue (`GameplayStatics.LoadGameFromSlot` "1"))
  (bind _saveshildhp (message `/Game/Interfaces/BPI_TestSave.GetSaveShildMaxHP` _returnvalue))
  (if (== _saveshildhp 25)
    (`self.FinishTest` "Succeeded" "Shield HP test successfull")
    (else
      (`self.FinishTest` "Failed" "Shield HP test failed"))))

(fn `IsReady`
  (returns (ReturnValue :type Boolean))
  (return (`KismetSystemLibrary.IsValid` (`GameplayStatics.GetPlayerCharacter` 0))))

(fn `UserConstructionScript`)