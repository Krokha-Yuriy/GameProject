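; BP_2StationDamege is a functional test that reports a station's HP after damage.
; An actor begin-overlap event gets the HP message from the overlapped actor, logs it and finishes the test as Succeeded without checking the value.
; The prepare, start and tick events are disabled, and the shield and station max-HP getters are stubs returning zero.
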(event `self.Actor.OnActorBeginOverlap`
  (params (OverlappedActor :type "Actor Object Reference") (OtherActor :type "Actor Object Reference"))
  (bind _stationhp (message `/Game/Interfaces/BPI_Test.GetStationHP` OverlappedActor))
  (`self.LogMessage` (`KismetStringLibrary.Concat_StrStr` "Station HP after damage:" (`KismetStringLibrary.Conv_DoubleToString` _stationhp)))
  (`self.FinishTest` "Succeeded"))

(fn `GetSaveShildMaxHP`
  (returns (SaveShildHP :type Integer))
  (return 0))

(fn `GetSaveStationMaxHP`
  (returns (SaveStationHP :type Integer))
  (return 0))

(fn `UserConstructionScript`
  (`parent.UserConstructionScript`))