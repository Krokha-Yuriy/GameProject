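; Functional test Blueprint that checks that projectiles carry the expected base damage.
; On StartTest it waits briefly, then gathers every actor tagged "Progectile" (spelled that way) and reads each one's damage through GetProjecttileDamageMessage.
; FinishTest is called inside the loop, passing on the base value and failing otherwise, so it never fires if no tagged actor exists.
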(event `self.ReceiveStartTest`
  (bind _returnvalue (`KismetSystemLibrary.GetDisplayName` self))
  (`KismetSystemLibrary.Delay` 1.0)
  (bind _outactors (`GameplayStatics.GetAllActorsWithTag` "Progectile"))
  (for _array_element _outactors
    (bind _basicdamage (message `/Game/Interfaces/BPI_Test.GetProjecttileDamage` _array_element))
    (if (== _basicdamage 1.0)
      (`self.LogMessage` (`KismetStringLibrary.Concat_StrStr` "Projectile damege: " (`KismetStringLibrary.Conv_DoubleToString` _basicdamage)))
      (`self.FinishTest` "Succeeded" (`KismetStringLibrary.Concat_StrStr` "Test passed:" _returnvalue))
      (else
        (`self.FinishTest` "Failed" (`KismetStringLibrary.Concat_StrStr` "Damage in not Base equal" _returnvalue))))))

(fn `UserConstructionScript`
  (`parent.UserConstructionScript`))