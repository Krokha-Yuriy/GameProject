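; Functional test that checks the damage value reported by projectiles in the level.
; It reports ready once a valid player character exists, waits briefly after starting, then gathers actors tagged "Progectile" (spelled that way).
; Each actor's ProjectileMessage result is compared to the expected damage, finishing the test as succeeded or failed.
; FinishTest sits inside the loop, so finding no tagged actors never finishes the test.
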(event `self.ReceiveStartTest`
  (`KismetSystemLibrary.Delay` 1.0)
  (bind _outactors (`GameplayStatics.GetAllActorsWithTag` "Progectile"))
  (for _array_element _outactors
    (bind _damage (message `/Game/Interfaces/BPI_Test.Projectile` _array_element))
    (if (== _damage 1.0)
      (`self.FinishTest` "Succeeded" "Damage is valid")
      (else
        (`self.FinishTest` "Failed" "Damage is not valid")))))

(fn `IsReady`
  (returns (ReturnValue :type Boolean))
  (return (`KismetSystemLibrary.IsValid` (`GameplayStatics.GetPlayerCharacter` 0))))

(fn `UserConstructionScript`)