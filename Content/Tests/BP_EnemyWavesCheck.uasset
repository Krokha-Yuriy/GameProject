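; BP_EnemyWavesCheck is a functional test that checks enemy waves spawn, becoming ready once a valid player character exists.
; StartTest looks up actors by enemy-type tag in timed sequence, then restarts the level and reports success.
; CheckEnemy fails the test only for an invalid actor among those found, so an empty result raises no failure.
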(event `self.ReceiveStartTest`
  (`self.CheckEnemy` "Pyr")
  (`KismetSystemLibrary.Delay` 15.0)
  (`self.CheckEnemy` "Arach")
  (`KismetSystemLibrary.Delay` 5.0)
  (`self.CheckEnemy` "Tank")
  (`KismetSystemLibrary.Delay` 5.0)
  (`self.CheckEnemy` "Mecha")
  (`KismetSystemLibrary.ExecuteConsoleCommand` "restartlevel" null)
  (`self.FinishTest` "Succeeded" "All enemies has been spawned"))

(fn `CheckEnemy`
  (params (Tag :type Name))
  (bind _outactors (`GameplayStatics.GetAllActorsWithTag` Tag))
  (for _array_element _outactors
    (`/Engine/EditorBlueprintResources/StandardMacros.IsValid` _array_element
      (:`Is Valid`
        (`KismetSystemLibrary.PrintString` "Enemy spawned"))
      (:`Is Not Valid`
        (`self.FinishTest` "Failed" "Cant find enemy")))))

(fn `IsReady`
  (returns (ReturnValue :type Boolean))
  (return (`KismetSystemLibrary.IsValid` (`GameplayStatics.GetPlayerCharacter` 0))))

(fn `UserConstructionScript`)