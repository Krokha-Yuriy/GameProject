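; Functional test that checks whether the Pyr, Arach, Tank and Mecha enemy types spawn during play.
; StartTest checks each tag in turn with delays between, then finishes as succeeded.
; CheckEnemys logs the first valid tagged actor and fails only on an invalid one, so an empty result passes silently.
; Meanwhile, a delayed Tick repeatedly destroys all actors with those tags.
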(event `self.ReceiveStartTest`
  (`parent.ReceiveStartTest`)
  (`self.CheckEnemys` "Pyr")
  (`KismetSystemLibrary.Delay` 15.0)
  (`self.CheckEnemys` "Arach")
  (`KismetSystemLibrary.Delay` 5.0)
  (`self.CheckEnemys` "Tank")
  (`KismetSystemLibrary.Delay` 5.0)
  (`self.CheckEnemys` "Mecha")
  (`self.FinishTest` "Succeeded" (`KismetSystemLibrary.GetDisplayName` self)))

(event `self.ReceiveTick`
  (params (DeltaSeconds :type "Float (single-precision)"))
  (`parent.ReceiveTick` DeltaSeconds)
  (`KismetSystemLibrary.Delay` 9.0)
  (`self.KillEnemys` "Pyr")
  (`self.KillEnemys` "Arach")
  (`self.KillEnemys` "Tank")
  (`self.KillEnemys` "Mecha"))

(fn `CheckEnemys`
  (params (Tag :type Name))
  (bind _outactors (`GameplayStatics.GetAllActorsWithTag` Tag))
  (for _array_element _outactors
    (`/Engine/EditorBlueprintResources/StandardMacros.IsValid` _array_element
      (:`Is Valid`
        (bind _returnvalue (`KismetStringLibrary.Concat_StrStr` "Enemy spawn:" (`KismetSystemLibrary.GetDisplayName` _array_element)))
        (`self.LogMessage` _returnvalue)
        (`KismetSystemLibrary.PrintString` _returnvalue)
        (return))
      (:`Is Not Valid`
        (`self.LogMessage` (`KismetStringLibrary.Concat_StrStr` "Not enemy spawn:" (`KismetSystemLibrary.GetDisplayName` _array_element)))
        (`self.FinishTest` "Failed")))))

(fn `KillEnemys`
  (params (Tag :type Name))
  (bind _outactors (`GameplayStatics.GetAllActorsWithTag` Tag))
  (for _array_element _outactors
    (`self.K2_DestroyActor` _array_element)))

(fn `UserConstructionScript`
  (`parent.UserConstructionScript`))